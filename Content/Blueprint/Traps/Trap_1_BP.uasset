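; Floor spike trap that springs when player character 0 steps into its FloorBox trigger.
; Spikes start hidden, then appear and rise with an eased MoveComponentTo.
; Leaving FloorBox hides them immediately as they sink back down more slowly.
; A separate Box overlap applies Damage to player pawn 0, without checking which actor overlapped.
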(event OnComponentBeginOverlap(FloorBox)
  (params (OverlappedComponent :type Primitive%20Component%20Object%20Reference) (OtherActor :type Actor%20Object%20Reference) (OtherComp :type Primitive%20Component%20Object%20Reference) (OtherBodyIndex :type Integer) (bFromSweep :type Boolean) (SweepResult :type Hit%20Result%20Structure%20%28by%20ref%29))
  (bind _spikes (Variables|Default|GetSpikes))
  (if (== OtherActor (Game|GetPlayerCharacter 0))
    (Components|MoveComponentTo _spikes "0.000000,0.000000, 0" "0, 0, 0" true true 0.5 false)
    (Development|SetHiddeninGame _spikes false false)))

(event OnComponentEndOverlap(FloorBox)
  (params (OverlappedComponent :type Primitive%20Component%20Object%20Reference) (OtherActor :type Actor%20Object%20Reference) (OtherComp :type Primitive%20Component%20Object%20Reference) (OtherBodyIndex :type Integer))
  (bind _spikes (Variables|Default|GetSpikes))
  (if (== OtherActor (Game|GetPlayerCharacter 0))
    (Components|MoveComponentTo _spikes "0.000000, 0,-170.000000" "0, 0, 0" true true 0.9 false)
    (Development|SetHiddeninGame _spikes true false)))

(event OnComponentBeginOverlap(Box)
  (params (OverlappedComponent :type Primitive%20Component%20Object%20Reference) (OtherActor :type Actor%20Object%20Reference) (OtherComp :type Primitive%20Component%20Object%20Reference) (OtherBodyIndex :type Integer) (bFromSweep :type Boolean) (SweepResult :type Hit%20Result%20Structure%20%28by%20ref%29))
  (Game|Damage|ApplyDamage (Game|Player|GetPlayerPawn 0) (Variables|Default|GetDamage) 0 0))

(event EventBeginPlay
  (Development|SetHiddeninGame (Variables|Default|GetSpikes) true false))

(fn ConstructionScript)