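; Trap actor with two spike wheels that start hidden, spin in opposite directions every tick, and hurt the player on contact.
; The player's first overlap with Box3 fires a one-shot that eases both wheels through a move and unhides them.
; Box and Box1 apply random damage to the player after a short delay, then toggle their collision off and on, which allows repeated overlap hits.
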(event OnComponentBeginOverlap(Box3)
  (params (OverlappedComponent :type Primitive%20Component%20Object%20Reference) (OtherActor :type Actor%20Object%20Reference) (OtherComp :type Primitive%20Component%20Object%20Reference) (OtherBodyIndex :type Integer) (bFromSweep :type Boolean) (SweepResult :type Hit%20Result%20Structure%20%28by%20ref%29))
  (if (== OtherActor (Game|GetPlayerCharacter 0))
    (Utilities|FlowControl|DoOnce false
      (:Completed
        (Components|MoveComponentTo (Variables|Default|GetSpike%20Wheel%202) "0, 0, 0" "0, 0, 0" true true 1.0 false)
        (Components|MoveComponentTo (Variables|Default|GetSpike%20Wheel%201) "0, 0, 0" "0, 0, 0" true true 1.0 false)
        (Development|SetHiddeninGame (Variables|Default|GetSpike%20Wheel%201) false false)))))

(event OnComponentBeginOverlap(Box1)
  (params (OverlappedComponent :type Primitive%20Component%20Object%20Reference) (OtherActor :type Actor%20Object%20Reference) (OtherComp :type Primitive%20Component%20Object%20Reference) (OtherBodyIndex :type Integer) (bFromSweep :type Boolean) (SweepResult :type Hit%20Result%20Structure%20%28by%20ref%29))
  (bind _box1 (Variables|Default|GetBox1))
  (if (== OtherActor (Game|GetPlayerCharacter 0))
    (Utilities|FlowControl|Delay 0.2)
    (Collision|SetCollisionEnabled _box1 "QueryAndPhysics")
    (Game|Damage|ApplyDamage (Game|Player|GetPlayerPawn 0) (Math|Random|RandomFloatinRange 5.0 15.0) 0 0)
    (Utilities|FlowControl|Delay 0.3)
    (Collision|SetCollisionEnabled _box1 "NoCollision")
    (Utilities|FlowControl|Delay 0.3)
    (Collision|SetCollisionEnabled _box1 "QueryAndPhysics")))

(event OnComponentBeginOverlap(Box)
  (params (OverlappedComponent :type Primitive%20Component%20Object%20Reference) (OtherActor :type Actor%20Object%20Reference) (OtherComp :type Primitive%20Component%20Object%20Reference) (OtherBodyIndex :type Integer) (bFromSweep :type Boolean) (SweepResult :type Hit%20Result%20Structure%20%28by%20ref%29))
  (bind _box (Variables|Default|GetBox))
  (if (== OtherActor (Game|GetPlayerCharacter 0))
    (Utilities|FlowControl|Delay 0.2)
    (Collision|SetCollisionEnabled _box "QueryAndPhysics")
    (Game|Damage|ApplyDamage (Game|Player|GetPlayerPawn 0) (Math|Random|RandomFloatinRange 5.0 15.0) 0 0)
    (Utilities|FlowControl|Delay 0.3)
    (Collision|SetCollisionEnabled _box "NoCollision")
    (Utilities|FlowControl|Delay 0.3)
    (Collision|SetCollisionEnabled _box "QueryAndPhysics")))

(event EventTick
  (params (DeltaSeconds :type Float%20%28single-precision%29))
  (Transformation|AddLocalRotation (Variables|Default|GetSpike%20Wheel%201) (Math|Rotator|MakeRotator 0.0 0.0 (* DeltaSeconds 1e+02)) false false)
  (Transformation|AddLocalRotation (Variables|Default|GetSpike%20Wheel%202) (Math|Rotator|MakeRotator 0.0 0.0 (* DeltaSeconds -1e+02)) false false))

(event EventBeginPlay
  (Development|SetHiddeninGame (Variables|Default|GetSpike%20Wheel%201) true false))

(fn ConstructionScript)