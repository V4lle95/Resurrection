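; Spike ball trap that swings around an anchor and hurts the player on contact.
; Each tick it pitches the Ancher component at a frame-rate-independent speed set by MultiplyRotation, with sweep enabled.
; When the Sphere begins overlapping the player character, it applies random damage between the Damage variable and a hardcoded upper limit.
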(event OnComponentBeginOverlap(Sphere)
  (params (OverlappedComponent :type Primitive%20Component%20Object%20Reference) (OtherActor :type Actor%20Object%20Reference) (OtherComp :type Primitive%20Component%20Object%20Reference) (OtherBodyIndex :type Integer) (bFromSweep :type Boolean) (SweepResult :type Hit%20Result%20Structure%20%28by%20ref%29))
  (if (== OtherActor (Game|GetPlayerCharacter 0))
    (Game|Damage|ApplyDamage (Game|Player|GetPlayerPawn 0) (Math|Random|RandomFloatinRange (Variables|Default|GetDamage) 7e+01) 0 0)))

(event EventTick
  (params (DeltaSeconds :type Float%20%28single-precision%29))
  (Transformation|AddLocalRotation (Variables|Default|GetAncher) (Math|Rotator|MakeRotator 0.0 (* DeltaSeconds (Variables|Default|GetMultiply%20rotation)) 0.0) true false))

(fn ConstructionScript)