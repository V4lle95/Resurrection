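; Weight-activated pressure plate whose Button component sinks when the player or an object of the ModelsForDoors class enters its Box trigger.
; Only the ModelsForDoors object also spawns ObjectToSpawn at the SPawner transform, once the press and a configurable DelayTime have finished.
; When either leaves the box, the Button eases back to its rest position, with no check for other occupants.
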(event OnComponentBeginOverlap(Box)
  (params (OverlappedComponent :type Primitive%20Component%20Object%20Reference) (OtherActor :type Actor%20Object%20Reference) (OtherComp :type Primitive%20Component%20Object%20Reference) (OtherBodyIndex :type Integer) (bFromSweep :type Boolean) (SweepResult :type Hit%20Result%20Structure%20%28by%20ref%29))
  (if (== OtherActor (Game|GetPlayerCharacter 0))
    (Components|MoveComponentTo (Variables|Default|GetButton) "0.000000, 0,-15.000000" "0, 0, 0" true true 2.0 false)
    (elif (== (Utilities|GetClass OtherActor) (Variables|Default|GetModels%20for%20Doors))
      (Components|MoveComponentTo (Variables|Default|GetButton) "0.000000, 0,-15.000000" "0, 0, 0" true true 2.0 false)
      (Utilities|FlowControl|Delay (Variables|Default|GetDelay%20Time))
      (Game|SpawnActorfromClass (Variables|Default|GetObject%20to%20spawn) (Transformation|GetWorldTransform (Variables|Default|GetSPawner)) "Undefined" 0 0))))

(event OnComponentEndOverlap(Box)
  (params (OverlappedComponent :type Primitive%20Component%20Object%20Reference) (OtherActor :type Actor%20Object%20Reference) (OtherComp :type Primitive%20Component%20Object%20Reference) (OtherBodyIndex :type Integer))
  (if (== OtherActor (Game|GetPlayerCharacter 0))
    (Components|MoveComponentTo (Variables|Default|GetButton) "0, 0,0.000000" "0, 0, 0" true true 1.0 false :!label _label)
    (elif (== (Utilities|GetClass OtherActor) (Variables|Default|GetModels%20for%20Doors))
      (goto _label))))

(fn ConstructionScript)